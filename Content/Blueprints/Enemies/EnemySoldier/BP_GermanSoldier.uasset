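; German soldier enemy that chases the player on sight, shoots at targets and reports its death to the spawn system.
; Pawn sensing drives an AI move toward the player, with the weapon attached to a mesh socket at BeginPlay.
; A separately triggered shoot event waits, plays muzzle FX and line traces, applying damage only if the target component is hit.
; Tick polls Health, notifying the cached BP_SpawnSystem and destroying the actor at zero.
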(event OnSeePawn(PawnSensing)
  (params (Pawn :type Pawn%20Object%20Reference))
  ;[1 1 1] Move To Players Location
  (bind _asbp_player_pawn (Utilities|Casting|CastToBP_PlayerPawn Pawn))
  (AI|AIMoveTo self "0, 0, 0" _asbp_player_pawn 3e+02 false))

(event Custom|Stoot%20Enemy
  (params (Enemy%20To%20Shoot :type Capsule%20Component%20Object%20Reference))
  (Utilities|FlowControl|Delay 5.0)
  (CallFunction|PlayShootingFX)
  (bind (_outhit _returnvalue) (Collision|LineTraceByChannel (Transformation|GetActorLocation) (+ (Transformation|GetWorldLocation Enemy%20To%20Shoot) "0, 0,60.000000") "TraceTypeQuery1" false 0 "ForDuration"))
  (if _returnvalue
    (if (== (.HitComponent (Collision|BreakHitResult _outhit)) Enemy%20To%20Shoot)
      (Game|Damage|ApplyDamage (.HitActor (Collision|BreakHitResult _outhit)) 2e+01 (Pawn|GetController) self "/Script/Engine.DamageType"))))

(event Custom|Play%20Shooting_FX
  (bind _weapon (Variables|Default|GetWeapon))
  ;[1 1 1] Play gun effect
  (Utilities|FlowControl|Delay 5.0)
  (Effects|SpawnEmitteratLocation "/Game/StarterContent/Particles/P_Explosion.P_Explosion" (Transformation|GetSocketLocation _weapon "Socket") (Transformation|GetSocketRotation _weapon "Socket") "0.500000,0.500000,0.500000"))

(event EventBeginPlay
  (Transformation|AttachComponentToComponent (Variables|Default|GetWeapon) (Variables|Character|GetMesh) "WeaponSocket" "KeepRelative" "SnapToTarget" "KeepRelative" true)
  (bind _outactors (Actor|GetAllActorsOfClass "/Game/Blueprints/Enemies/BP_SpawnSystem.BP_SpawnSystem_C"))
  (Variables|Default|SetSpawn%20System (Utilities|Array|Get(acopy) _outactors))
  (Development|PrintString "Found"))

(event Collision|EventActorBeginOverlap
  (params (OtherActor :type Actor%20Object%20Reference)))

(event EventTick
  (params (DeltaSeconds :type Float%20%28single-precision%29))
  (if (<= (Variables|Default|Gethealth) 0)
    (bind _asbp_spawn_system (Utilities|Casting|CastToBP_SpawnSystem (Variables|Default|GetSpawn%20System)))
    (Default|EnemyKilled _asbp_spawn_system)
    (Actor|DestroyActor)))

(fn ConstructionScript)