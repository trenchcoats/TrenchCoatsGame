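; German medic enemy AI that wanders the navmesh and heals the player.
; On BeginPlay it loops AI MoveTo toward random nearby navigable points.
; Pawn sensing stores a sighted player pawn as the move's target actor, which is never cleared afterwards.
; Each successful move restarts the loop, adds clamped health to that stored player and prints the value; the full-health branch does nothing.
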(event OnSeePawn(PawnSensing)
  (params (Pawn :type Pawn%20Object%20Reference))
  (bind _asbp_player_pawn (Utilities|Casting|CastToBP_PlayerPawn Pawn))
  (AI|AIMoveTo self (.RandomLocation (Class|NavigationSystemV1|GetRandomPointinNavigableRadius (Transformation|GetActorLocation) 5e+02 0 0)) _asbp_player_pawn 5.0 false
    (:OnSuccess
      (CallFunction|MovetoRandomLocation self)
      (Variables|/Script/TrenchCoatsGame.PlayerPawn|SetcurrentPlayerHealth _asbp_player_pawn (Math|Conversions|ToFloat(Integer) (Math|Integer|Clamp(Integer) (+ (Math|Float|Truncate (Variables|/Script/TrenchCoatsGame.PlayerPawn|GetcurrentPlayerHealth _asbp_player_pawn)) 10) 0 100)))
      (Development|PrintString (Utilities|String|ToString(Integer) (Math|Float|Truncate (Variables|/Script/TrenchCoatsGame.PlayerPawn|GetcurrentPlayerHealth _asbp_player_pawn))))
      (if (>= (Math|Float|Truncate (Variables|/Script/TrenchCoatsGame.PlayerPawn|GetcurrentPlayerHealth _asbp_player_pawn)) 100)
        _))))

(event Custom|MoveToRandomLocation
  (AI|AIMoveTo self (.RandomLocation (Class|NavigationSystemV1|GetRandomPointinNavigableRadius (Transformation|GetActorLocation) 5e+02 0 0)) (stale OnSeePawn(PawnSensing) _asbp_player_pawn) 5.0 false
    (:OnSuccess
      (CallFunction|MovetoRandomLocation self)
      (Variables|/Script/TrenchCoatsGame.PlayerPawn|SetcurrentPlayerHealth (stale OnSeePawn(PawnSensing) _asbp_player_pawn) (Math|Conversions|ToFloat(Integer) (Math|Integer|Clamp(Integer) (+ (Math|Float|Truncate (Variables|/Script/TrenchCoatsGame.PlayerPawn|GetcurrentPlayerHealth (stale OnSeePawn(PawnSensing) _asbp_player_pawn))) 10) 0 100)))
      (Development|PrintString (Utilities|String|ToString(Integer) (Math|Float|Truncate (Variables|/Script/TrenchCoatsGame.PlayerPawn|GetcurrentPlayerHealth (stale OnSeePawn(PawnSensing) _asbp_player_pawn)))))
      (if (>= (Math|Float|Truncate (Variables|/Script/TrenchCoatsGame.PlayerPawn|GetcurrentPlayerHealth (stale OnSeePawn(PawnSensing) _asbp_player_pawn))) 100)
        _))))

(event EventBeginPlay
  (CallFunction|MovetoRandomLocation))

(event Collision|EventActorBeginOverlap
  (params (OtherActor :type Actor%20Object%20Reference)))

(event EventTick
  (params (DeltaSeconds :type Float%20%28single-precision%29)))

(fn ConstructionScript)