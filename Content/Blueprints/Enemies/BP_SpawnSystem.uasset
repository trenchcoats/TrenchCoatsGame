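; Wave spawner that releases German soldier and medic AI over three configured waves.
; Tick sets the wave's quotas, picks a random spawn-point component (RandomInteger(2) never reaches the third), and spawns through five-second Delays.
; Exhausted quotas zero NumberSpawned, so waves advance after spawning without waiting for kills.
; The Tick logic is marked for rework; EnemySpawn is an uncalled soldier-only variant, and EnemyKilled's graph call is unwired.
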(event EventTick
  (params (DeltaSeconds :type Float%20%28single-precision%29))
  ;[1 1 1] REWORK THIS
  (Utilities|FlowControl|Sequence
    (:then_0
      (if (Variables|Default|GetWaveStarted)
        (switch int (Variables|Default|GetCurrentWave)
          (:1
            (Variables|Default|SetNumberOfSoldiersToSpawn 1)
            (Variables|Default|SetNumberOfMedicsToSpawn 0)
            (Variables|Default|SetNumberSpawned 10))
          (:2
            (Variables|Default|SetNumberOfSoldiersToSpawn 1)
            (Variables|Default|SetNumberOfMedicsToSpawn 1)
            (Variables|Default|SetNumberSpawned 2))
          (:3
            (Variables|Default|SetNumberOfSoldiersToSpawn 15)
            (Variables|Default|SetNumberOfMedicsToSpawn 5)
            (Variables|Default|SetNumberSpawned 20)))
        (Variables|Default|SetWaveStarted false)))
    (:then_1
      (switch int (Math|Random|RandomInteger 2)
        (:0
          (Variables|Default|SetLocation (Transformation|GetWorldLocation (Variables|Default|GetSpawnPoint1))))
        (:1
          (Variables|Default|SetLocation (Transformation|GetWorldLocation (Variables|Default|GetSpawnPoint2))))
        (:2
          (Variables|Default|SetLocation (Transformation|GetWorldLocation (Variables|Default|GetSpawnPoint3))))))
    (:then_2
      (Utilities|FlowControl|Delay 5.0)
      (Utilities|FlowControl|Sequence
        (:then_0
          (if (> (Variables|Default|GetNumberOfSoldiersToSpawn) 0)
            (AI|SpawnAIFromClass "/Game/Blueprints/Enemies/EnemySoldier/BP_GermanSoldier.BP_GermanSoldier_C" 0 (Variables|Default|GetLocation) "0, 0, 0" false)
            (Variables|Default|SetNumberOfSoldiersToSpawn (- (Variables|Default|GetNumberOfSoldiersToSpawn) 1))))
        (:then_1
          (if (> (Variables|Default|GetNumberOfMedicsToSpawn) 0)
            (AI|SpawnAIFromClass "/Game/Blueprints/Enemies/BP_GermanMedicV2.BP_GermanMedicV2_C" 0 (Variables|Default|GetLocation) "0, 0, 0" false)
            (Variables|Default|SetNumberOfMedicsToSpawn (- (Variables|Default|GetNumberOfMedicsToSpawn) 1))))))
    (:then_3
      (if (== (Variables|Default|GetNumberOfSoldiersToSpawn) 0)
        (if (== (Variables|Default|GetNumberOfMedicsToSpawn) 0)
          (Variables|Default|SetNumberSpawned 0))))
    (:then_4
      (if (== (Variables|Default|GetNumberSpawned) 0)
        (Utilities|FlowControl|Delay 5.0)
        (if (< (Variables|Default|GetCurrentWave) 4)
          (Variables|Default|SetCurrentWave (+ (Variables|Default|GetCurrentWave) 1))
          (Variables|Default|SetWaveStarted true))))))

(fn ConstructionScript)

(fn EnemySpawn
  (Utilities|FlowControl|Sequence
    (:then_0
      (if (Variables|Default|GetWaveStarted)
        (switch int (Variables|Default|GetCurrentWave)
          (:1
            (Variables|Default|SetNumberOfSoldiersToSpawn 5))
          (:2
            (Variables|Default|SetNumberOfSoldiersToSpawn 10))
          (:3
            (Variables|Default|SetNumberOfSoldiersToSpawn 15))
          (:4
            (Variables|Default|SetNumberOfSoldiersToSpawn 20))
          (:5
            (Variables|Default|SetNumberOfSoldiersToSpawn 25)))
        (Variables|Default|SetWaveStarted false)
        (else
          (if (> (Variables|Default|GetNumberOfSoldiersToSpawn) 0) :!label _label
            (AI|SpawnAIFromClass "/Game/Blueprints/Enemies/EnemySoldier/BP_GermanSoldier.BP_GermanSoldier_C" 0 "0, 0,288.000000" "0, 0, 0" false)
            (Variables|Default|SetNumberOfSoldiersToSpawn (- (Variables|Default|GetCurrentWave) 1))))))
    (:then_1
      (goto _label))))

(fn EnemyKilled
  (Variables|Default|SetNumberSpawned (- (Variables|Default|GetNumberSpawned) 1)))