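; BP_EnemyTest is a test enemy that wanders the navmesh and pursues the player once PawnSensing spots them.
; A single AI MoveTo serves both: it takes a random nearby point and the cached player as target, which is never cleared.
; Each successful move restarts the loop, raises the player's health by a clamped step and prints it, with no check that a player was seen.
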(event OnSeePawn(PawnSensing)
  (params (Pawn :type Pawn%20Object%20Reference))
  (bind _asplayer_pawn (Utilities|Casting|CastToPlayerPawn Pawn))
  (AI|AIMoveTo 0 (.RandomLocation (Class|NavigationSystemV1|GetRandomPointinNavigableRadius (Transformation|GetActorLocation) 5e+02 0 0)) _asplayer_pawn 5.0 false
    (:OnSuccess
      (CallFunction|MovetoRandomLocation self)
      (bind _output_get (Variables|/Script/TrenchCoatsGame.PlayerPawn|SetcurrentPlayerHealth _asplayer_pawn (Math|Conversions|ToFloat(Integer) (Math|Integer|Clamp(Integer) (+ (Math|Float|Truncate (Variables|/Script/TrenchCoatsGame.PlayerPawn|GetcurrentPlayerHealth _asplayer_pawn)) 10) 0 100))))
      (Development|PrintString (Utilities|String|ToString(Float) _output_get))
      (if (>= (Math|Float|Truncate (Variables|/Script/TrenchCoatsGame.PlayerPawn|GetcurrentPlayerHealth _asplayer_pawn)) 100)
        _))))

(event Custom|MoveToRandomLocation
  (AI|AIMoveTo 0 (.RandomLocation (Class|NavigationSystemV1|GetRandomPointinNavigableRadius (Transformation|GetActorLocation) 5e+02 0 0)) (stale OnSeePawn(PawnSensing) _asplayer_pawn) 5.0 false
    (:OnSuccess
      (CallFunction|MovetoRandomLocation self)
      (bind _output_get (Variables|/Script/TrenchCoatsGame.PlayerPawn|SetcurrentPlayerHealth (stale OnSeePawn(PawnSensing) _asplayer_pawn) (Math|Conversions|ToFloat(Integer) (Math|Integer|Clamp(Integer) (+ (Math|Float|Truncate (Variables|/Script/TrenchCoatsGame.PlayerPawn|GetcurrentPlayerHealth (stale OnSeePawn(PawnSensing) _asplayer_pawn))) 10) 0 100))))
      (Development|PrintString (Utilities|String|ToString(Float) _output_get))
      (if (>= (Math|Float|Truncate (Variables|/Script/TrenchCoatsGame.PlayerPawn|GetcurrentPlayerHealth (stale OnSeePawn(PawnSensing) _asplayer_pawn))) 100)
        _))))

(event EventBeginPlay
  (CallFunction|MovetoRandomLocation))

(event Collision|EventActorBeginOverlap
  (params (OtherActor :type Actor%20Object%20Reference)))

(fn ConstructionScript)