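; BP_GermanMedicV2 is an enemy AI pawn that wanders the navmesh and pursues the player once seen; no healing logic is present.
; A self-restarting AIMoveTo picks nearby random points, and PawnSensing re-enters it with the sighted player stored as target actor, which is never cleared.
; Tick polls Health and, at zero or below, notifies the BP_SpawnSystem found at BeginPlay of the kill and destroys the actor.
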(event OnSeePawn(PawnSensing)
  (params (Pawn :type Pawn%20Object%20Reference))
  (bind _asbp_player_pawn (Utilities|Casting|CastToBP_PlayerPawn Pawn))
  (AI|AIMoveTo self (.RandomLocation (Class|NavigationSystemV1|GetRandomPointinNavigableRadius (Transformation|GetActorLocation) 5e+02 0 0)) _asbp_player_pawn 2e+01 false
    (:OnSuccess
      (CallFunction|MovetoRandomLocation self))))

(event Custom|MoveToRandomLocation
  (AI|AIMoveTo self (.RandomLocation (Class|NavigationSystemV1|GetRandomPointinNavigableRadius (Transformation|GetActorLocation) 5e+02 0 0)) (stale OnSeePawn(PawnSensing) _asbp_player_pawn) 2e+01 false
    (:OnSuccess
      (CallFunction|MovetoRandomLocation self))))

(event EventBeginPlay
  (bind _outactors (Actor|GetAllActorsOfClass "/Game/Blueprints/Enemies/BP_SpawnSystem.BP_SpawnSystem_C"))
  (Variables|Default|SetSpawnSystem (Utilities|Array|Get(acopy) _outactors))
  (CallFunction|MovetoRandomLocation))

(event EventTick
  (params (DeltaSeconds :type Float%20%28single-precision%29))
  (if (<= (Variables|Default|Gethealth) 0)
    (bind _asbp_spawn_system (Utilities|Casting|CastToBP_SpawnSystem (Variables|Default|GetSpawnSystem)))
    (Default|EnemyKilled _asbp_spawn_system)
    (Actor|DestroyActor)))

(fn ConstructionScript)