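; BP_RifleHolster is a player rifle holster that attaches a BP_FrenchRifle left within its volume.
; Each Tick runs a narrow box overlap at the Box component for physics-body rifles, with Hand in the ignore list.
; When the player pawn's RiflePickedUp is false, the first rifle found attaches to Box, keeping its world location and rotation rather than snapping.
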(event EventBeginPlay)

(event Collision|EventActorBeginOverlap
  (params (OtherActor :type Actor%20Object%20Reference)))

(event EventTick
  (params (DeltaSeconds :type Float%20%28single-precision%29))
  (bind (_outactors _returnvalue) (Collision|BoxOverlapActors (Transformation|GetWorldLocation (Variables|Default|GetBox)) "70.000000,6.000000,10.000000" (Utilities|Array|MakeArray "ObjectTypeQuery4") "/Game/Blueprints/Weapons/FrenchRifle/BP_FrenchRifle.BP_FrenchRifle_C" (Utilities|Array|MakeArray (Variables|Default|GetHand) 0 0) :!class /Script/Engine.KismetSystemLibrary))
  (if _returnvalue
    (bind _asbp_player_pawn (Utilities|Casting|CastToBP_PlayerPawn (Game|Player|GetPlayerPawn 0)))
    (if (not (Variables|/Script/TrenchCoatsGame.PlayerPawn|GetriflePickedUp _asbp_player_pawn))
      (Transformation|AttachComponentToComponent (Variables|/Script/Engine.Actor|GetRootComponent (Utilities|Array|Get(acopy) _outactors)) (Variables|Default|GetBox) "None" "KeepWorld" "KeepWorld" "KeepRelative" true))))

(fn ConstructionScript)