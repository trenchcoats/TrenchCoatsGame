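; BP_AmmoPack is a player ammo pouch that spawns ammo when a VR motion controller reaches into it.
; Each Tick, a small box overlap checks for BP_MotionControllerNormal.
; It spawns a pistol mag, or rifle ammo if only the rifle is picked up, at the mesh location.
; The stored AmmoSpawned reference blocks repeat spawns until the overlap ends and clears it, without destroying the ammo.
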(event EventTick
  (params (DeltaSeconds :type Float%20%28single-precision%29))
  (bind _returnvalue (Collision|BoxOverlapActors (Transformation|GetWorldLocation (Variables|Default|GetBox)) "2.500000,5.000000,4.000000" (Utilities|Array|MakeArray "ObjectTypeQuery2") "/Game/VirtualRealityBP/Blueprints/BP_MotionControllerNormal.BP_MotionControllerNormal_C" (Utilities|Array|MakeArray (Variables|Default|GetPistol) (Variables|Default|GetRifle) (Variables|Default|GetHolster) (Variables|Default|GetRifleHolster) (Variables|Default|GetHealthPack)) :!class /Script/Engine.KismetSystemLibrary))
  (if _returnvalue
    (if (not (== (Utilities|GetClass (Variables|Default|GetAmmoSpawned)) "/Game/Blueprints/Weapons/FrenchRifle/BP_FrenchRifleAmmoPack.BP_FrenchRifleAmmoPack_C"))
      (if (not (== (Utilities|GetClass (Variables|Default|GetAmmoSpawned)) "/Game/Blueprints/Weapons/Ruby/BP_EmptyPistolMag.BP_EmptyPistolMag_C"))
        (bind _asbp_player_pawn (Utilities|Casting|CastToBP_PlayerPawn (Game|Player|GetPlayerPawn 0)))
        (if (Variables|/Script/TrenchCoatsGame.PlayerPawn|GetpistolPickedUp _asbp_player_pawn)
          (Variables|Default|SetAmmoToSpawn "/Game/Blueprints/Weapons/Ruby/BP_EmptyPistolMag.BP_EmptyPistolMag_C")
          (bind _returnvalue_2 (Game|SpawnActorfromClass (Variables|Default|GetAmmoToSpawn) (Math|Conversions|ToTransform(Vector) (Transformation|GetWorldLocation (Variables|Default|GetStaticMesh))) "Undefined" 0 0 :!label _label))
          (Variables|Default|SetAmmoSpawned _returnvalue_2)
          (elif (Variables|/Script/TrenchCoatsGame.PlayerPawn|GetriflePickedUp _asbp_player_pawn)
            (Variables|Default|SetAmmoToSpawn "/Game/Blueprints/Weapons/FrenchRifle/BP_FrenchRifleAmmoPack.BP_FrenchRifleAmmoPack_C")
            (goto _label)))))
    (else
      (Variables|Default|SetAmmoSpawned 0))))

(fn ConstructionScript)