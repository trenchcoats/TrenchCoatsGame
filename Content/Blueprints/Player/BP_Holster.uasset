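; BP_Holster is a player holster that holds a BP_RubyPistol when it is not picked up.
; Every Tick it runs a small box overlap at its Box component for physics-body pistols, with Hand in the ignore list.
; When one is found and BP_PlayerPawn's PistolPickedUp is false, it attaches the pistol's root to the Box, keeping world location and rotation rather than snapping.
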(event EventTick
  (params (DeltaSeconds :type Float%20%28single-precision%29))
  (bind (_outactors _returnvalue) (Collision|BoxOverlapActors (Transformation|GetWorldLocation (Variables|Default|GetBox)) "5.000000,5.000000,5.000000" (Utilities|Array|MakeArray "ObjectTypeQuery4") "/Game/Blueprints/Weapons/Ruby/BP_RubyPistol.BP_RubyPistol_C" (Utilities|Array|MakeArray (Variables|Default|GetHand) 0 0) :!class /Script/Engine.KismetSystemLibrary))
  (if _returnvalue
    (bind _asbp_player_pawn (Utilities|Casting|CastToBP_PlayerPawn (Game|Player|GetPlayerPawn 0)))
    (if (not (Variables|/Script/TrenchCoatsGame.PlayerPawn|GetpistolPickedUp _asbp_player_pawn))
      (Transformation|AttachComponentToComponent (Variables|/Script/Engine.Actor|GetRootComponent (Utilities|Array|Get(acopy) _outactors)) (Variables|Default|GetBox) "None" "KeepWorld" "KeepWorld" "KeepRelative" true))))

(fn ConstructionScript)