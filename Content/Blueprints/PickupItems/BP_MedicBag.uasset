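; BP_MedicBag is a medic bag item that the player can pick up and drop.
; Pickup turns off mesh physics and attaches the bag to the supplied component with a small offset, while Drop detaches it and re-enables physics.
; Both events set a PickedUp flag, which Tick copies every frame to MedicBagPickedUp on the first player's BP_PlayerPawn.
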(event EventBeginPlay)

(event Collision|EventActorBeginOverlap
  (params (OtherActor :type Actor%20Object%20Reference)))

(event EventTick
  (params (DeltaSeconds :type Float%20%28single-precision%29))
  (bind _returnvalue (Game|Player|GetPlayerPawn 0))
  ;[1 1 1] Checks if Pistol has been picked up or not
  (if (Variables|Default|GetpickedUp)
    (bind _asbp_player_pawn (Utilities|Casting|CastToBP_PlayerPawn _returnvalue))
    (Variables|/Script/TrenchCoatsGame.PlayerPawn|SetmedicBagPickedUp _asbp_player_pawn true)
    (else
      (bind _asbp_player_pawn_2 (Utilities|Casting|CastToBP_PlayerPawn _returnvalue))
      (Variables|/Script/TrenchCoatsGame.PlayerPawn|SetmedicBagPickedUp _asbp_player_pawn_2 false))))

(event EventDrop
  ;[1 1 1] Pick up
  (Variables|Default|SetpickedUp false)
  (Physics|SetSimulatePhysics (Variables|Default|GetmedicBagMeshComponent) true)
  (Transformation|DetachFromActor "KeepWorld" "KeepWorld" "KeepWorld"))

(event EventPickup
  (params (AttachTo :type Scene%20Component%20Object%20Reference))
  ;[1 1 1] Pick up
  (Variables|Default|SetpickedUp true)
  (Physics|SetSimulatePhysics (Variables|Default|GetmedicBagMeshComponent) false)
  (Transformation|AttachComponentToComponent (VehicleSound|GetRootComponent) AttachTo "None" "SnapToTarget" "SnapToTarget" "KeepWorld" false)
  (Transformation|SetRelativeLocationAndRotation (Variables|Default|GetmedicBagMeshComponent) "0,-1.000000, 0" "0, 0, 0" false false))

(fn ConstructionScript)