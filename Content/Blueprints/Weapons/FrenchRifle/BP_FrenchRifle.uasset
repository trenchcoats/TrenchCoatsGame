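; BP_FrenchRifle is a VR rifle that motion controllers pick up, drop and steady with a second hand.
; Pickup attaches it to the first hand; a trigger registers the second, releasing it on end overlap depending on grip state.
; Tick updates pawn flags, aims the mesh from first hand to second using first-hand roll, and snaps an unheld rifle to an overlapping BP_RifleHolster.
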(event OnComponentBeginOverlap(SecondHandTrigger)
  (params (OverlappedComponent :type Primitive%20Component%20Object%20Reference) (OtherActor :type Actor%20Object%20Reference) (OtherComp :type Primitive%20Component%20Object%20Reference) (OtherBodyIndex :type Integer) (bFromSweep :type Boolean) (SweepResult :type Hit%20Result%20Structure%20%28by%20ref%29))
  ;[1 1 1] Second Hand Stick
  (if (Variables|Default|GetFirstHandGrabbed)
    (bind _asbp_motion_controller_normal (Utilities|Casting|CastToBP_MotionControllerNormal OtherActor))
    (if (!= (Variables|/Game/VirtualRealityBP/Blueprints/BP_MotionControllerNormal.BP_MotionControllerNormal_C|GetMotionController _asbp_motion_controller_normal) (Variables|Default|GetFirstHand))
      (Variables|Default|SetsecondHandGrabbed true)
      (Variables|Default|SetSecondHand (Variables|/Game/VirtualRealityBP/Blueprints/BP_MotionControllerNormal.BP_MotionControllerNormal_C|GetMotionController _asbp_motion_controller_normal)))))

(event OnComponentEndOverlap(SecondHandTrigger)
  (params (OverlappedComponent :type Primitive%20Component%20Object%20Reference) (OtherActor :type Actor%20Object%20Reference) (OtherComp :type Primitive%20Component%20Object%20Reference) (OtherBodyIndex :type Integer))
  ;[1 1 1] Second Hand Stick
  (if (Variables|Default|GetsecondHandGrabbed)
    (Utilities|IsValid (Variables|Default|GetSecondHand)
      (:Is%20Valid
        (if (and (.bSuccess (Utilities|Casting|CastToBP_MotionControllerNormal (Components|GetOwner (Variables|Default|GetSecondHand)))) (Utilities|Enum|NotEqual(Enum) (Variables|/Game/VirtualRealityBP/Blueprints/BP_MotionControllerNormal.BP_MotionControllerNormal_C|GetGripState (.AsBP%20Motion%20Controller%20Normal (Utilities|Casting|CastToBP_MotionControllerNormal (Components|GetOwner (Variables|Default|GetSecondHand))))) "NewEnumerator2"))
          (Variables|Default|SetsecondHandGrabbed false :!label _label)
          (Variables|Default|SetSecondHand 0)
          (Transformation|SetRelativeRotation (Variables|Default|GetrifleMesh) (Variables|Default|GetOneHandRotation) false false)))
      (:Is%20Not%20Valid
        (goto _label)))))

(event EventBeginPlay)

(event Collision|EventActorBeginOverlap
  (params (OtherActor :type Actor%20Object%20Reference)))

(event EventTick
  (params (DeltaSeconds :type Float%20%28single-precision%29))
  (bind _returnvalue (Game|Player|GetPlayerPawn 0))
  (bind _returnvalue_2 (Game|Player|GetPlayerPawn 0))
  (bind _pickedup (Variables|Default|GetpickedUp))
  (bind _secondhand (Variables|Default|GetSecondHand))
  (bind _firsthand (Variables|Default|GetFirstHand))
  (bind _returnvalue_3 (Transformation|GetWorldLocation _secondhand))
  (bind _returnvalue_4 (Transformation|GetWorldLocation _firsthand))
  (bind _returnvalue_5 (Math|Rotator|FindLookatRotation _returnvalue_4 _returnvalue_3))
  (bind (_roll _pitch _yaw) (Math|Rotator|BreakRotator _returnvalue_5))
  (Utilities|FlowControl|Sequence
    (:then_0
      ;[1 1 1] Checking if Rifle has been picked up or not
      (if _pickedup
        (bind _asmotion_controller_pawn (Utilities|Casting|CastToMotionControllerPawn _returnvalue_2))
        (Variables|/Game/VirtualRealityBP/Blueprints/MotionControllerPawn.MotionControllerPawn_C|SetRifle _asmotion_controller_pawn true)
        (else
          (Utilities|Casting|CastToMotionControllerPawn _returnvalue_2))))
    (:then_1
      (if _pickedup
        (bind _asbp_player_pawn (Utilities|Casting|CastToBP_PlayerPawn _returnvalue))
        (Variables|/Script/TrenchCoatsGame.PlayerPawn|SetriflePickedUp _asbp_player_pawn true)
        (else
          (bind _asbp_player_pawn_2 (Utilities|Casting|CastToBP_PlayerPawn _returnvalue))
          (Variables|/Script/TrenchCoatsGame.PlayerPawn|SetriflePickedUp _asbp_player_pawn_2 false))))
    (:then_2
      ;[1 1 1] Rotation Check
      (Utilities|FlowControl|Sequence
        (:then_0
          (if (and (Variables|Default|GetsecondHandGrabbed) (Utilities|IsValid (Variables|Default|GetSecondHand)))
            (Transformation|SetWorldRotation (Variables|Default|GetrifleMesh) (Math|Rotator|MakeRotator (.Roll (Math|Rotator|BreakRotator (Transformation|GetWorldRotation _firsthand))) _pitch _yaw) false false)))))
    (:then_3
      (bind (_outactors _returnvalue_6) (Collision|BoxOverlapActors (Transformation|GetWorldLocation (Variables|Default|GetBox)) "2.300000,0.200000,0.300000" (Utilities|Array|MakeArray "ObjectTypeQuery2") "/Game/Blueprints/Player/BP_RifleHolster.BP_RifleHolster_C" (Utilities|Array|MakeArray (Variables|Default|GetHand) 0 0) :!class /Script/Engine.KismetSystemLibrary))
      (if _returnvalue_6
        (if (not (Variables|Default|GetpickedUp))
          (Transformation|AttachActorToActor (Utilities|Array|Get(acopy) _outactors) "None" "SnapToTarget" "SnapToTarget" "KeepWorld" true))))))

(event EventDrop
  ;[1 1 1] Picking Up And Dropping Rifle
  (Variables|Default|SetpickedUp false)
  (Physics|SetSimulatePhysics (Variables|Default|GetrifleMesh) true)
  (Transformation|DetachFromActor "KeepWorld" "KeepWorld" "KeepWorld")
  (Variables|Default|SetfirstHandGrabbed false)
  (Variables|Default|SetsecondHandGrabbed false))

(event EventPickup
  (params (AttachTo :type Scene%20Component%20Object%20Reference))
  ;[1 1 1] Picking Up And Dropping Rifle
  (if (not (Variables|Default|GetfirstHandGrabbed))
    (Variables|Default|SetpickedUp true)
    (Physics|SetSimulatePhysics (Variables|Default|GetrifleMesh) false)
    (Transformation|AttachComponentToComponent (VehicleSound|GetRootComponent) AttachTo "None" "SnapToTarget" "SnapToTarget" "KeepWorld" false)
    (Transformation|SetRelativeRotation (Variables|Default|GetrifleMesh) (Variables|Default|GetOneHandRotation) false false)
    (Variables|Default|SetcurrentHand (Components|GetOwner AttachTo))
    (Variables|Default|SetfirstHandGrabbed true)
    (Variables|Default|SetsecondHandGrabbed false)
    (Variables|Default|SetFirstHand AttachTo)))

(fn ConstructionScript)