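; BP_FrenchRifleAmmoPack is a grabbable ammo pack that reloads the French rifle on contact.
; On spawn it scales down, disables physics and destroys itself if not held after three seconds.
; Pickup snaps it to the given component at a fixed offset, and Drop detaches it with physics enabled.
; Each Tick a small box overlap looks for BP_FrenchRifle, calls Reload on it and destroys the pack.
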(event EventBeginPlay
  ;[1 1 1] When Ammo is spawned
  (Transformation|SetActorScale3D "0.600000,0.600000,0.600000")
  (Physics|SetSimulatePhysics (Variables|Default|GetFrenchRifleAmmoPack) false)
  (Utilities|FlowControl|Delay 3.0)
  (if (not (Variables|Default|GetPickedUp))
    (Actor|DestroyActor)))

(event EventTick
  (params (DeltaSeconds :type Float%20%28single-precision%29))
  ;[1 1 1] Loading Ammo in Rifle
  (bind (_outactors _returnvalue) (Collision|BoxOverlapActors (Transformation|GetWorldLocation (Variables|Default|GetBox)) "5.000000,5.000000,5.000000" (Utilities|Array|MakeArray "ObjectTypeQuery4") "/Game/Blueprints/Weapons/FrenchRifle/BP_FrenchRifle.BP_FrenchRifle_C" (Utilities|Array|MakeArray (Variables|Default|GetHand)) :!class /Script/Engine.KismetSystemLibrary))
  (if _returnvalue
    (if (== (Utilities|GetClass (Utilities|Array|Get(acopy) _outactors)) "/Game/Blueprints/Weapons/FrenchRifle/BP_FrenchRifle.BP_FrenchRifle_C")
      (bind _asbp_french_rifle (Utilities|Casting|CastToBP_FrenchRifle (Utilities|Array|Get(acopy) _outactors)))
      (Class|FrenchRifle|Reload _asbp_french_rifle)
      (Actor|DestroyActor)
      (Development|PrintString "Reloaded"))))

(event EventDrop
  ;[1 1 1] Picking Up Ammo
  (Variables|Default|SetpickedUp false)
  (Physics|SetSimulatePhysics (Variables|Default|GetFrenchRifleAmmoPack) true)
  (Transformation|DetachFromActor "KeepWorld" "KeepWorld" "KeepWorld"))

(event EventPickup
  (params (AttachTo :type Scene%20Component%20Object%20Reference))
  ;[1 1 1] Picking Up Ammo
  (Variables|Default|SetpickedUp true)
  (Physics|SetSimulatePhysics (Variables|Default|GetFrenchRifleAmmoPack) false)
  (Transformation|AttachComponentToComponent (VehicleSound|GetRootComponent) AttachTo "None" "SnapToTarget" "SnapToTarget" "KeepWorld" false)
  (Transformation|SetRelativeLocationAndRotation (Variables|Default|GetFrenchRifleAmmoPack) "6.000000,0.000000,0.000000" "0.000000,90.000000,90.000000" false false))

(fn ConstructionScript)