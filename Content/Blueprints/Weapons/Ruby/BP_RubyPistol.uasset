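; Ruby pistol actor for motion-controller play that can be picked up, dropped and holstered.
; Pickup and Drop toggle physics and attachment to the hand, while Tick copies the held state to the player pawns.
; When not held, a per-tick box overlap snaps it onto a nearby BP_Holster.
; Left and right fire inputs only disable the muzzle flash emitter, with no shot or ray cast implemented.
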(event EventTick
  (params (DeltaSeconds :type Float%20%28single-precision%29))
  (bind _returnvalue (Game|Player|GetPlayerPawn 0))
  (bind _returnvalue_2 (Game|Player|GetPlayerPawn 0))
  (bind _pickedup (Variables|Default|GetpickedUp))
  (Utilities|FlowControl|Sequence
    (:then_0
      ;[1 1 1] Checks if Pistol has been picked up or not
      (if _pickedup
        (bind _asmotion_controller_pawn (Utilities|Casting|CastToMotionControllerPawn _returnvalue_2))
        (Variables|/Game/VirtualRealityBP/Blueprints/MotionControllerPawn.MotionControllerPawn_C|SetPistol _asmotion_controller_pawn true)
        (else
          (Utilities|Casting|CastToMotionControllerPawn _returnvalue_2))))
    (:then_1
      (if _pickedup
        (bind _asbp_player_pawn (Utilities|Casting|CastToBP_PlayerPawn _returnvalue))
        (Variables|/Script/TrenchCoatsGame.PlayerPawn|SetpistolPickedUp _asbp_player_pawn true)
        (else
          (bind _asbp_player_pawn_2 (Utilities|Casting|CastToBP_PlayerPawn _returnvalue))
          (Variables|/Script/TrenchCoatsGame.PlayerPawn|SetpistolPickedUp _asbp_player_pawn_2 false))))
    (:then_2
      (bind (_outactors _returnvalue_3) (Collision|BoxOverlapActors (Transformation|GetWorldLocation (Variables|Default|GetBox)) "5.000000,5.000000,5.000000" (Utilities|Array|MakeArray "ObjectTypeQuery2") "/Game/Blueprints/Player/BP_Holster.BP_Holster_C" (Utilities|Array|MakeArray (Variables|Default|GetHand) 0 0) :!class /Script/Engine.KismetSystemLibrary))
      (if _returnvalue_3
        (if (not (Variables|Default|GetpickedUp))
          (Transformation|AttachActorToActor (Utilities|Array|Get(acopy) _outactors) "None" "SnapToTarget" "SnapToTarget" "KeepWorld" true))))))

(event EventDrop
  ;[1 1 1] Picking up Code
  (Variables|Default|SetpickedUp false)
  (Physics|SetSimulatePhysics (Variables|Default|GetpistolMesh) true)
  (Transformation|DetachFromActor "KeepWorld" "KeepWorld" "KeepWorld"))

(event EventPickup
  (params (AttachTo :type Scene%20Component%20Object%20Reference))
  ;[1 1 1] Picking up Code
  (Variables|Default|SetpickedUp true)
  (Physics|SetSimulatePhysics (Variables|Default|GetpistolMesh) false)
  (Transformation|AttachComponentToComponent (VehicleSound|GetRootComponent) AttachTo "None" "SnapToTarget" "SnapToTarget" "KeepWorld" false)
  (Transformation|SetRelativeLocationAndRotation (Variables|Default|GetpistolMesh) "0,0.000000,3.000000" "0.000000,-90.000000,-90.000000" false false)
  (Variables|Default|SetcurrentHand (Components|GetOwner AttachTo)))

(event Input|ActionEvents|InputActionFireLeft
  (params (Key :type Key%20Structure))
  ;[1 1 1] Ray-Casting
  (:Pressed
    (Utilities|FlowControl|Sequence
      (:then_0
        (if (Variables|Default|GetpickedUp)
          (Utilities|Casting|CastToBP_PlayerPawn (Game|Player|GetPlayerPawn 0))))
      (:then_1
        (Effects|Components|ParticleSystem|SetEmitterEnable (Variables|Default|GetP_MuzzleFlash) "None" false)))))

(event Input|ActionEvents|InputActionFireRight
  (params (Key :type Key%20Structure))
  ;[1 1 1] Ray-Casting
  (:Pressed
    (Utilities|FlowControl|Sequence
      (:then_0
        (if (Variables|Default|GetpickedUp)
          (Utilities|Casting|CastToBP_PlayerPawn (Game|Player|GetPlayerPawn 0))))
      (:then_1
        (Effects|Components|ParticleSystem|SetEmitterEnable (Variables|Default|GetP_MuzzleFlash) "None" false)))))

(fn ConstructionScript)