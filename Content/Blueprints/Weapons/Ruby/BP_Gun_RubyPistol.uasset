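; BP_Gun_RubyPistol is a Ruby pistol weapon actor that can be picked up and dropped.
; Pickup disables physics on the RubyPistol component, snaps the actor's root to the supplied component and slightly offsets RubyPistol.
; Drop re-enables physics and detaches the actor in place, with both events updating the PickedUp flag.
; Tick prints AmmoClip every frame as debug output; this graph contains no firing logic.
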(event EventBeginPlay)

(event Collision|EventActorBeginOverlap
  (params (OtherActor :type Actor%20Object%20Reference)))

(event EventTick
  (params (DeltaSeconds :type Float%20%28single-precision%29))
  (Development|PrintString (Utilities|String|ToString(Integer) (Variables|Default|GetammoClip))))

(event EventPickup
  (params (AttachTo :type Scene%20Component%20Object%20Reference))
  (Variables|Default|SetpickedUp true)
  (Physics|SetSimulatePhysics (Variables|Default|GetRubyPistol) false)
  (Transformation|AttachComponentToComponent (VehicleSound|GetRootComponent) AttachTo "None" "SnapToTarget" "SnapToTarget" "KeepWorld" false)
  (Transformation|SetRelativeLocationAndRotation (Variables|Default|GetRubyPistol) "0,-1.000000, 0" "0, 0, 0" false false))

(event EventDrop
  (Variables|Default|SetpickedUp false)
  (Physics|SetSimulatePhysics (Variables|Default|GetRubyPistol) true)
  (Transformation|DetachFromActor "KeepWorld" "KeepWorld" "KeepWorld"))

(fn ConstructionScript)