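; BP_EmptyPistolMag is a pistol magazine actor that can be picked up, dropped and loaded into BP_RubyPistol.
; On spawn it rescales, disables physics and destroys itself if not held when a three-second delay ends.
; Pickup snaps it to the given component, while Drop detaches it and enables physics.
; Each tick, a small box overlap checks for a pistol, calls its Reload and destroys the magazine.
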(event EventBeginPlay
  ;[1 1 1] When Ammo is spawned
  (Transformation|SetActorScale3D "1.800000,2.000000,3.000000")
  (Physics|SetSimulatePhysics (Variables|Default|GetPistolmag) false)
  (Utilities|FlowControl|Delay 3.0)
  (if (not (Variables|Default|GetPickedUp))
    (Actor|DestroyActor)))

(event EventTick
  (params (DeltaSeconds :type Float%20%28single-precision%29))
  ;[1 1 1] Loading Ammo into Pistol
  (bind (_outactors _returnvalue) (Collision|BoxOverlapActors (Transformation|GetWorldLocation (Variables|Default|GetBox)) "5.000000,5.000000,5.000000" (Utilities|Array|MakeArray "ObjectTypeQuery4") "/Game/Blueprints/Weapons/Ruby/BP_RubyPistol.BP_RubyPistol_C" (Utilities|Array|MakeArray (Variables|Default|GetHand)) :!class /Script/Engine.KismetSystemLibrary))
  (if _returnvalue
    (if (== (Utilities|GetClass (Utilities|Array|Get(acopy) _outactors)) "/Game/Blueprints/Weapons/Ruby/BP_RubyPistol.BP_RubyPistol_C")
      (bind _asbp_ruby_pistol (Utilities|Casting|CastToBP_RubyPistol (Utilities|Array|Get(acopy) _outactors)))
      (Class|RubyPistol|Reload _asbp_ruby_pistol)
      (Actor|DestroyActor)
      (Development|PrintString "Reloaded"))))

(event EventDrop
  ;[1 1 1] Ammo Pick Up
  (Variables|Default|SetpickedUp false)
  (Physics|SetSimulatePhysics (Variables|Default|GetPistolmag) true)
  (Transformation|DetachFromActor "KeepWorld" "KeepWorld" "KeepWorld"))

(event EventPickup
  (params (AttachTo :type Scene%20Component%20Object%20Reference))
  ;[1 1 1] Ammo Pick Up
  (Variables|Default|SetpickedUp true)
  (Physics|SetSimulatePhysics (Variables|Default|GetPistolmag) false)
  (Transformation|AttachComponentToComponent (VehicleSound|GetRootComponent) AttachTo "None" "SnapToTarget" "SnapToTarget" "KeepWorld" false)
  (Transformation|SetRelativeLocationAndRotation (Variables|Default|GetPistolmag) "-3.000000,0.000000,0.000000" "90.000000, 0,90.000000" false false))

(fn ConstructionScript)